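; Trader NPC that the player can trade with, pickpocket while crouching, or loot when dead.
; Interact opens trade or container widgets accordingly, trading only in blackboard State 0, and Fill writes slots back, re-adding equipment withheld from stealing.
; Save data extends the parent's with trade stock and gold.
; BeginPlay polls until the game loads, then outside first load restores state by ID, ragdolling dead traders or passing saved AI data to the controller.
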(event `self.ReceiveBeginPlay`
  (set `self.MyAnimBP` (cast `/Game/ThirdPerson/Blueprints/Animations/ABP_MyAnimBP` (`SkeletalMeshComponent.GetAnimInstance` (`self.Mesh`)) :!pure true))
  (`KismetSystemLibrary.K2_SetTimer` null "RecoverStamina" 0.1 true)
  (bind _asbp_third_person_game_mode (cast `/Game/ThirdPerson/Blueprints/BP_ThirdPersonGameMode` (`GameplayStatics.GetGameMode`)))
  (if (`/Game/ThirdPerson/Blueprints/BP_ThirdPersonGameMode.GameLoaded?` _asbp_third_person_game_mode) :!label _label
    (if (not (`/Game/ThirdPerson/Blueprints/BP_ThirdPersonGameMode.FirstLoad?` _asbp_third_person_game_mode))
      (bind _asbp_game_instance (cast `/Game/ThirdPerson/Blueprints/BP_GameInstance` (`GameplayStatics.GetGameInstance`)))
      (for _array_element (`/Game/ThirdPerson/Blueprints/BP_GameInstance.HumansSaveDataArray` _asbp_game_instance)
        (bind (_id _dead_ _transform _health _maxhealth _stamina _maxstamina _mana _maxmana _level _inventoryarray _wasfalling_ _startlocation _teamnumber _aicsavedata _endurance _melee _ranged _armor _sneak _agility _speech _destruction _restoration _conjuration _tradearray _tradergold) (break `/Game/ThirdPerson/Blueprints/EnumsStructures/Structs/Save/Structure_HumanSaveData` _array_element))
        (if (== _id (`self.ID`))
          (`self.K2_SetActorTransform` _transform false true)
          (set `self.Health` _health)
          (set `self.MaxHealth` _maxhealth)
          (set `self.Stamina` _stamina)
          (set `self.MaxStamina` _maxstamina)
          (set `self.Mana` _mana)
          (set `self.MaxMana` _maxmana)
          (set `self.Level` _level)
          (set `self.Endurance` _endurance)
          (set `self.Melee` _melee)
          (set `self.Ranged` _ranged)
          (set `self.Armor` _armor)
          (set `self.Sneak` _sneak)
          (set `self.Agility` _agility)
          (set `self.Speech` _speech)
          (set `self.Destruction` _destruction)
          (set `self.Restoration` _restoration)
          (set `self.Conjuration` _conjuration)
          (set `self.InventoryArray` _inventoryarray)
          (`self.ChangeArmor`)
          (set `self.WasFalling` _wasfalling_)
          (set `self.StartLocation` _startlocation)
          (set `self.TeamNumber` _teamnumber)
          (set `self.TradeArray` _tradearray)
          (set `self.TraderGold` _tradergold)
          (if _dead_
            (set `self.Dead?` true)
            (`Controller.UnPossess` (`self.GetController`))
            (`PrimitiveComponent.SetSimulatePhysics` (`self.Mesh`) true)
            (`ActorComponent.K2_DestroyComponent` (`self.CapsuleComponent`))
            (break)
            (else
              (message `/Game/ThirdPerson/Blueprints/General/BPInterfaces/BPI_AIC.SetAICSaveData` (`self.GetController`) _aicsavedata)
              (break))))))
    (else
      (`KismetSystemLibrary.Delay` 0.0)
      (goto _label))))

(event `/Game/ThirdPerson/Blueprints/General/BPInterfaces/BPI_AI.Add/RemoveGold`
  (params (`GoldQuantity(+/-)` :type Integer))
  (set `self.TraderGold` (+ (`self.TraderGold`) `GoldQuantity(+/-)`)))

(event `/Game/ThirdPerson/Blueprints/General/BPInterfaces/BPI_Interact.Interact`
  (bind _returnvalue (`GameplayStatics.GetPlayerCharacter` 0))
  (bind _returnvalue_2 (`GameplayStatics.GetPlayerController` 0))
  (bind _returnvalue_3 (`GameplayStatics.GetPlayerController` 0))
  (bind _returnvalue_4 (`GameplayStatics.GetPlayerController` 0))
  (bind _asbp_character (cast `/Game/ThirdPerson/Blueprints/BP_Character` (`GameplayStatics.GetPlayerCharacter` 0) :!pure true))
  (bind _asbp_character_2 (cast `/Game/ThirdPerson/Blueprints/BP_Character` (`GameplayStatics.GetPlayerCharacter` 0) :!pure true))
  (bind _asbp_character_3 (cast `/Game/ThirdPerson/Blueprints/BP_Character` (`GameplayStatics.GetPlayerCharacter` 0) :!pure true))
  (bind _tradewidget (`/Game/ThirdPerson/Blueprints/BP_Character.TradeWidget` _asbp_character_2))
  (bind _inventorywidget (`/Game/ThirdPerson/Blueprints/BP_Character.InventoryWidget` _asbp_character_2))
  (bind _containerwidget (`/Game/ThirdPerson/Blueprints/BP_Character.ContainerWidget` _asbp_character_3))
  (bind _containerwidget_2 (`/Game/ThirdPerson/Blueprints/BP_Character.ContainerWidget` _asbp_character))
  (bind _tradewidget_2 (`/Game/ThirdPerson/Blueprints/BP_Character.TradeWidget` (cast `/Game/ThirdPerson/Blueprints/BP_Character` _returnvalue :!pure true)))
  (if (`self.Dead?`)
    (if (not (or (`Widget.IsInViewport` _containerwidget) (`Widget.IsInViewport` (`/Game/ThirdPerson/Blueprints/BP_Character.EquipmentWidget` _asbp_character_3))))
      (`Widget.RemoveFromParent` (`/Game/ThirdPerson/Blueprints/BP_Character.InventoryWidget` _asbp_character_3))
      (`UserWidget.AddToViewport` _containerwidget 0)
      (`UserWidget.AddToViewport` (`/Game/ThirdPerson/Blueprints/BP_Character.InventoryWidget` _asbp_character_3) 0)
      (set `/Game/ThirdPerson/Blueprints/Widgets/Interfaces/W_Container.ContainerName` (`self.HumanName`) _containerwidget)
      (`/Game/ThirdPerson/Blueprints/Widgets/Interfaces/W_BaseInterface.FillInterface` (`/Game/ThirdPerson/Blueprints/BP_Character.ContainerWidget` (cast `/Game/ThirdPerson/Blueprints/BP_Character` (`GameplayStatics.GetPlayerCharacter` 0) :!pure true)) (`self.InventoryArray`))
      (set `PlayerController.bShowMouseCursor` true _returnvalue_2)
      (`WidgetBlueprintLibrary.SetInputMode_GameAndUIEx` _returnvalue_2 null))
    (elif (`/Game/ThirdPerson/Blueprints/BP_Character.IsCrouching` (cast `/Game/ThirdPerson/Blueprints/BP_Character` (`GameplayStatics.GetPlayerCharacter` 0) :!pure true))
      (if (not (or (`Widget.IsInViewport` _containerwidget_2) (`Widget.IsInViewport` (`/Game/ThirdPerson/Blueprints/BP_Character.EquipmentWidget` _asbp_character))))
        (`Widget.RemoveFromParent` (`/Game/ThirdPerson/Blueprints/BP_Character.InventoryWidget` _asbp_character))
        (`UserWidget.AddToViewport` _containerwidget_2 0)
        (`UserWidget.AddToViewport` (`/Game/ThirdPerson/Blueprints/BP_Character.InventoryWidget` _asbp_character) 0)
        (set `/Game/ThirdPerson/Blueprints/Widgets/Interfaces/W_Container.ContainerName` (`self.HumanName`) _containerwidget_2)
        (bind _stealinventoryarray (`self.GetStealInventoryArray`))
        (`/Game/ThirdPerson/Blueprints/Widgets/Interfaces/W_BaseInterface.FillInterface` (`/Game/ThirdPerson/Blueprints/BP_Character.ContainerWidget` (cast `/Game/ThirdPerson/Blueprints/BP_Character` (`GameplayStatics.GetPlayerCharacter` 0) :!pure true)) _stealinventoryarray)
        (set `PlayerController.bShowMouseCursor` true _returnvalue_4)
        (`WidgetBlueprintLibrary.SetInputMode_GameAndUIEx` _returnvalue_4 null))
      (elif (== (`BlackboardComponent.GetValueAsInt` (`AIBlueprintHelperLibrary.GetBlackboard` null) "State") 0)
        (if (not (or (`Widget.IsInViewport` _tradewidget) (`Widget.IsInViewport` (`/Game/ThirdPerson/Blueprints/BP_Character.EquipmentWidget` _asbp_character_2))))
          (`Widget.RemoveFromParent` _inventorywidget)
          (`UserWidget.AddToViewport` _inventorywidget 0)
          (`UserWidget.AddToViewport` _tradewidget 0)
          (set `/Game/ThirdPerson/Blueprints/Widgets/Interfaces/W_Trade.TraderName` (`self.HumanName`) _tradewidget)
          (`/Game/ThirdPerson/Blueprints/Widgets/Interfaces/W_BaseInterface.FillInterface` (`/Game/ThirdPerson/Blueprints/BP_Character.TradeWidget` (cast `/Game/ThirdPerson/Blueprints/BP_Character` (`GameplayStatics.GetPlayerCharacter` 0) :!pure true)) (`self.TradeArray`))
          (bind _goldquantity (`/Game/ThirdPerson/Blueprints/General/BPInterfaces/BPI_AI.GetGold`))
          (`TextBlock.SetText` (`/Game/ThirdPerson/Blueprints/Widgets/Interfaces/W_Trade.TraderGold` _tradewidget_2) (`KismetTextLibrary.Conv_StringToText` (`KismetStringLibrary.Concat_StrStr` "Trader gold: " (`KismetStringLibrary.Conv_IntToString` _goldquantity))))
          (bind _goldquantity_2 (message `/Game/ThirdPerson/Blueprints/General/BPInterfaces/BPI_AI.GetGold` _returnvalue))
          (`TextBlock.SetText` (`/Game/ThirdPerson/Blueprints/Widgets/Interfaces/W_Trade.MyGold` _tradewidget_2) (`KismetTextLibrary.Conv_StringToText` (`KismetStringLibrary.Concat_StrStr` "Your gold: " (`KismetStringLibrary.Conv_IntToString` _goldquantity_2))))
          (set `PlayerController.bShowMouseCursor` true _returnvalue_3)
          (`WidgetBlueprintLibrary.SetInputMode_GameAndUIEx` _returnvalue_3 null))))))

(event `/Game/ThirdPerson/Blueprints/General/BPInterfaces/BPI_Interact.InteractText`
  (bind _interacttextwidget (`/Game/ThirdPerson/Blueprints/BP_Character.InteractTextWidget` (cast `/Game/ThirdPerson/Blueprints/BP_Character` (`GameplayStatics.GetPlayerCharacter` 0) :!pure true)))
  (bind _interacttextwidget_2 (`/Game/ThirdPerson/Blueprints/BP_Character.InteractTextWidget` (cast `/Game/ThirdPerson/Blueprints/BP_Character` (`GameplayStatics.GetPlayerCharacter` 0) :!pure true)))
  (bind _interacttextwidget_3 (`/Game/ThirdPerson/Blueprints/BP_Character.InteractTextWidget` (cast `/Game/ThirdPerson/Blueprints/BP_Character` (`GameplayStatics.GetPlayerCharacter` 0) :!pure true)))
  (if (`self.Dead?`)
    (`/Game/ThirdPerson/Blueprints/Widgets/UI/W_InteractText.UpdateInteractText` _interacttextwidget_3 "NewEnumerator2" (`self.HumanName`))
    (`UserWidget.AddToViewport` _interacttextwidget_3 0)
    (elif (`/Game/ThirdPerson/Blueprints/BP_Character.IsCrouching` (cast `/Game/ThirdPerson/Blueprints/BP_Character` (`GameplayStatics.GetPlayerCharacter` 0) :!pure true))
      (`/Game/ThirdPerson/Blueprints/Widgets/UI/W_InteractText.UpdateInteractText` _interacttextwidget "NewEnumerator3" (`self.HumanName`))
      (`UserWidget.AddToViewport` _interacttextwidget 0)
      (elif (== (`BlackboardComponent.GetValueAsInt` (`AIBlueprintHelperLibrary.GetBlackboard` null) "State") 0)
        (`/Game/ThirdPerson/Blueprints/Widgets/UI/W_InteractText.UpdateInteractText` _interacttextwidget_2 "NewEnumerator1" (`self.HumanName`))
        (`UserWidget.AddToViewport` _interacttextwidget_2 0)))))

(event `/Game/ThirdPerson/Blueprints/General/BPInterfaces/BPI_Interact.Fill`
  (if (`self.Dead?`)
    (`KismetArrayLibrary.Array_Clear` (`self.InventoryArray`))
    (for _array_element (`/Game/ThirdPerson/Blueprints/Widgets/Interfaces/W_BaseInterface.InterfaceSlotArray` (`/Game/ThirdPerson/Blueprints/BP_Character.ContainerWidget` (cast `/Game/ThirdPerson/Blueprints/BP_Character` (`GameplayStatics.GetPlayerCharacter` 0) :!pure true))) :!label _label_2
      (if (`/Game/ThirdPerson/Blueprints/Widgets/Slots/W_ContainerSlot.Filled?` _array_element)
        (`KismetArrayLibrary.Array_Add` (`self.InventoryArray`) (`/Game/ThirdPerson/Blueprints/Widgets/Slots/W_ContainerSlot.Item Info` _array_element))))
    (elif (`/Game/ThirdPerson/Blueprints/BP_Character.IsCrouching` (cast `/Game/ThirdPerson/Blueprints/BP_Character` (`GameplayStatics.GetPlayerCharacter` 0) :!pure true))
      (`KismetArrayLibrary.Array_Clear` (`self.InventoryArray`))
      (for _array_element_2 (`self.RemovedEquipmentArray`)
        (`KismetArrayLibrary.Array_Add` (`self.InventoryArray`) _array_element_2))
      (goto _label_2)
      (else
        (`KismetArrayLibrary.Array_Clear` (`self.TradeArray`))
        (for _array_element_3 (`/Game/ThirdPerson/Blueprints/Widgets/Interfaces/W_BaseInterface.InterfaceSlotArray` (`/Game/ThirdPerson/Blueprints/BP_Character.TradeWidget` (cast `/Game/ThirdPerson/Blueprints/BP_Character` (`GameplayStatics.GetPlayerCharacter` 0) :!pure true)))
          (if (`/Game/ThirdPerson/Blueprints/Widgets/Slots/W_TradeSlot.Filled?` _array_element_3)
            (`KismetArrayLibrary.Array_Add` (`self.TradeArray`) (`/Game/ThirdPerson/Blueprints/Widgets/Slots/W_TradeSlot.Item Info` _array_element_3))))))))

(fn `Get Save Data`
  (returns (`Human Save Data` :type "/Game/ThirdPerson/Blueprints/EnumsStructures/Structs/Save/Structure_HumanSaveData Structure"))
  (bind _human_save_data (`parent.Get Save Data`))
  (return (make `/Game/ThirdPerson/Blueprints/EnumsStructures/Structs/Save/Structure_HumanSaveData` (break `/Game/ThirdPerson/Blueprints/EnumsStructures/Structs/Save/Structure_HumanSaveData` _human_save_data) (`.Dead?_76_E228CA85491F7A782F429AB0E218EA28` (break `/Game/ThirdPerson/Blueprints/EnumsStructures/Structs/Save/Structure_HumanSaveData` _human_save_data)) (`.Transform_32_93E028B6454F69D9D8E7159892CB9FD6` (break `/Game/ThirdPerson/Blueprints/EnumsStructures/Structs/Save/Structure_HumanSaveData` _human_save_data)) (`.Health_2_68A96961478535C2D2AF20971396642C` (break `/Game/ThirdPerson/Blueprints/EnumsStructures/Structs/Save/Structure_HumanSaveData` _human_save_data)) (`.MaxHealth_103_7D9814F64EF5A241258DE3B87592D228` (break `/Game/ThirdPerson/Blueprints/EnumsStructures/Structs/Save/Structure_HumanSaveData` _human_save_data)) (`.Stamina_5_770D00A7435B79BA19A70F9724EF646F` (break `/Game/ThirdPerson/Blueprints/EnumsStructures/Structs/Save/Structure_HumanSaveData` _human_save_data)) (`.MaxStamina_104_03D96BFB4F91EF3247C76AACAB205281` (break `/Game/ThirdPerson/Blueprints/EnumsStructures/Structs/Save/Structure_HumanSaveData` _human_save_data)) (`.Mana_6_06E75B2E4C9AFEC761F8BBB13BFB7E43` (break `/Game/ThirdPerson/Blueprints/EnumsStructures/Structs/Save/Structure_HumanSaveData` _human_save_data)) (`.MaxMana_105_91271A734814F56458A59D834E88953D` (break `/Game/ThirdPerson/Blueprints/EnumsStructures/Structs/Save/Structure_HumanSaveData` _human_save_data)) (`.Level_10_C61BB3ED4561DE6C4F3A3398F40FF367` (break `/Game/ThirdPerson/Blueprints/EnumsStructures/Structs/Save/Structure_HumanSaveData` _human_save_data)) (`.InventoryArray_39_BA8CBA6842E37EB80171AD995C06272E` (break `/Game/ThirdPerson/Blueprints/EnumsStructures/Structs/Save/Structure_HumanSaveData` _human_save_data)) (`.WasFalling?_47_771D8C0C4FED65D228559F8E30177D17` (break `/Game/ThirdPerson/Blueprints/EnumsStructures/Structs/Save/Structure_HumanSaveData` _human_save_data)) (`.StartLocation_49_2FA9962F40098D9DD5F5B2800D087E81` (break `/Game/ThirdPerson/Blueprints/EnumsStructures/Structs/Save/Structure_HumanSaveData` _human_save_data)) (`.TeamNumber_56_1BA7434341236B13C9E8258CA45A6068` (break `/Game/ThirdPerson/Blueprints/EnumsStructures/Structs/Save/Structure_HumanSaveData` _human_save_data)) (`.AICSaveData_121_6820091742F8F4693D269D80A3E68B9A` (break `/Game/ThirdPerson/Blueprints/EnumsStructures/Structs/Save/Structure_HumanSaveData` _human_save_data)) (`.Endurance_79_AE24D74E447763081D4FB2ACB9DF6A50` (break `/Game/ThirdPerson/Blueprints/EnumsStructures/Structs/Save/Structure_HumanSaveData` _human_save_data)) (`.Melee_88_5ADF0F04465CA383B44C3FB2C52511D7` (break `/Game/ThirdPerson/Blueprints/EnumsStructures/Structs/Save/Structure_HumanSaveData` _human_save_data)) (`.Ranged_89_AA2B81804D1F1B0CAF3760AB95BDD9D1` (break `/Game/ThirdPerson/Blueprints/EnumsStructures/Structs/Save/Structure_HumanSaveData` _human_save_data)) (`.Armor_90_6022B1C6478950147C51E6AA33FF5526` (break `/Game/ThirdPerson/Blueprints/EnumsStructures/Structs/Save/Structure_HumanSaveData` _human_save_data)) (`.Sneak_107_53F82DD446FA9B1E09CD678746558008` (break `/Game/ThirdPerson/Blueprints/EnumsStructures/Structs/Save/Structure_HumanSaveData` _human_save_data)) (`.Agility_92_DA319720416E63C61D05CBB029DA543E` (break `/Game/ThirdPerson/Blueprints/EnumsStructures/Structs/Save/Structure_HumanSaveData` _human_save_data)) (`.Speech_93_EFFBA16649B0362C52F636B763E6604E` (break `/Game/ThirdPerson/Blueprints/EnumsStructures/Structs/Save/Structure_HumanSaveData` _human_save_data)) (`.Destruction_95_300A98154078F05AF0E4E2A225D06402` (break `/Game/ThirdPerson/Blueprints/EnumsStructures/Structs/Save/Structure_HumanSaveData` _human_save_data)) (`.Restoration_97_AA215B744048CD2E1DEFD195FF4225B5` (break `/Game/ThirdPerson/Blueprints/EnumsStructures/Structs/Save/Structure_HumanSaveData` _human_save_data)) (`.Conjuration_98_2DF1C4C242F4C3E299F3949DBF6D9546` (break `/Game/ThirdPerson/Blueprints/EnumsStructures/Structs/Save/Structure_HumanSaveData` _human_save_data)) (`self.TradeArray`) (`self.TraderGold`))))

(fn `GetFriendlyState`
  (params (InputTeamNumber :type Integer))
  (returns (FriendlyState :type Integer))
  (bind _teamnumber (`self.TeamNumber`))
  (if (== InputTeamNumber 0)
    (if (or (== _teamnumber 1) (== _teamnumber 2))
      (return 1)
      (else
        (return 0)))
    (elif (> InputTeamNumber 0)
      (return 0)
      (else
        (return -1)))))

(fn `GetGold`
  (returns (GoldQuantity :type Integer))
  (return (`self.TraderGold`)))

(fn `GetHealthAndDefence`
  (returns (Health :type "Float (double-precision)") (Defence :type "Float (double-precision)"))
  (return 0.0 0.0))

(fn `GetTeam`
  (returns (OutputTeamNumber :type Integer))
  (return (`self.TeamNumber`)))

(fn `UserConstructionScript`
  (`parent.UserConstructionScript`))