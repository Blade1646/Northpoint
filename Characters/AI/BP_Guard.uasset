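; Guard NPC that the player can loot when dead or pickpocket while crouching, with team-based attitude logic.
; Interact opens the player's container and inventory widgets with the full or stealable inventory, and InteractText shows the matching prompt.
; Fill rebuilds the inventory from widget slots, restoring removed equipment after pickpocketing.
; GetFriendlyState treats its own team as friendly, turns hostile to teams 0 and 1 when the player has a fine, and to negative teams.
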(event `/Game/ThirdPerson/Blueprints/General/BPInterfaces/BPI_Interact.Interact`
  (bind _returnvalue (`GameplayStatics.GetPlayerController` 0))
  (bind _returnvalue_2 (`GameplayStatics.GetPlayerController` 0))
  (bind _asbp_character (cast `/Game/ThirdPerson/Blueprints/BP_Character` (`GameplayStatics.GetPlayerCharacter` 0) :!pure true))
  (bind _asbp_character_2 (cast `/Game/ThirdPerson/Blueprints/BP_Character` (`GameplayStatics.GetPlayerCharacter` 0) :!pure true))
  (bind _containerwidget (`/Game/ThirdPerson/Blueprints/BP_Character.ContainerWidget` _asbp_character_2))
  (bind _containerwidget_2 (`/Game/ThirdPerson/Blueprints/BP_Character.ContainerWidget` _asbp_character))
  (if (`self.Dead?`)
    (if (not (or (`Widget.IsInViewport` _containerwidget) (`Widget.IsInViewport` (`/Game/ThirdPerson/Blueprints/BP_Character.EquipmentWidget` _asbp_character_2))))
      (`Widget.RemoveFromParent` (`/Game/ThirdPerson/Blueprints/BP_Character.InventoryWidget` _asbp_character_2))
      (`UserWidget.AddToViewport` _containerwidget 0)
      (`UserWidget.AddToViewport` (`/Game/ThirdPerson/Blueprints/BP_Character.InventoryWidget` _asbp_character_2) 0)
      (set `/Game/ThirdPerson/Blueprints/Widgets/Interfaces/W_Container.ContainerName` (`self.HumanName`) _containerwidget)
      (`/Game/ThirdPerson/Blueprints/Widgets/Interfaces/W_BaseInterface.FillInterface` (`/Game/ThirdPerson/Blueprints/BP_Character.ContainerWidget` (cast `/Game/ThirdPerson/Blueprints/BP_Character` (`GameplayStatics.GetPlayerCharacter` 0) :!pure true)) (`self.InventoryArray`))
      (set `PlayerController.bShowMouseCursor` true _returnvalue)
      (`WidgetBlueprintLibrary.SetInputMode_GameAndUIEx` _returnvalue null))
    (elif (`/Game/ThirdPerson/Blueprints/BP_Character.IsCrouching` (cast `/Game/ThirdPerson/Blueprints/BP_Character` (`GameplayStatics.GetPlayerCharacter` 0) :!pure true))
      (if (not (or (`Widget.IsInViewport` _containerwidget_2) (`Widget.IsInViewport` (`/Game/ThirdPerson/Blueprints/BP_Character.EquipmentWidget` _asbp_character))))
        (`Widget.RemoveFromParent` (`/Game/ThirdPerson/Blueprints/BP_Character.InventoryWidget` _asbp_character))
        (`UserWidget.AddToViewport` _containerwidget_2 0)
        (`UserWidget.AddToViewport` (`/Game/ThirdPerson/Blueprints/BP_Character.InventoryWidget` _asbp_character) 0)
        (set `/Game/ThirdPerson/Blueprints/Widgets/Interfaces/W_Container.ContainerName` (`self.HumanName`) _containerwidget_2)
        (bind _stealinventoryarray (`self.GetStealInventoryArray`))
        (`/Game/ThirdPerson/Blueprints/Widgets/Interfaces/W_BaseInterface.FillInterface` (`/Game/ThirdPerson/Blueprints/BP_Character.ContainerWidget` (cast `/Game/ThirdPerson/Blueprints/BP_Character` (`GameplayStatics.GetPlayerCharacter` 0) :!pure true)) _stealinventoryarray)
        (set `PlayerController.bShowMouseCursor` true _returnvalue_2)
        (`WidgetBlueprintLibrary.SetInputMode_GameAndUIEx` _returnvalue_2 null))
      (elif (== (`BlackboardComponent.GetValueAsInt` (`AIBlueprintHelperLibrary.GetBlackboard` null) "State") 0)
        _))))

(event `/Game/ThirdPerson/Blueprints/General/BPInterfaces/BPI_Interact.InteractText`
  (bind _interacttextwidget (`/Game/ThirdPerson/Blueprints/BP_Character.InteractTextWidget` (cast `/Game/ThirdPerson/Blueprints/BP_Character` (`GameplayStatics.GetPlayerCharacter` 0) :!pure true)))
  (bind _interacttextwidget_2 (`/Game/ThirdPerson/Blueprints/BP_Character.InteractTextWidget` (cast `/Game/ThirdPerson/Blueprints/BP_Character` (`GameplayStatics.GetPlayerCharacter` 0) :!pure true)))
  (bind _interacttextwidget_3 (`/Game/ThirdPerson/Blueprints/BP_Character.InteractTextWidget` (cast `/Game/ThirdPerson/Blueprints/BP_Character` (`GameplayStatics.GetPlayerCharacter` 0) :!pure true)))
  (if (`self.Dead?`)
    (`/Game/ThirdPerson/Blueprints/Widgets/UI/W_InteractText.UpdateInteractText` _interacttextwidget_2 "NewEnumerator2" (`self.HumanName`))
    (`UserWidget.AddToViewport` _interacttextwidget_2 0)
    (elif (`/Game/ThirdPerson/Blueprints/BP_Character.IsCrouching` (cast `/Game/ThirdPerson/Blueprints/BP_Character` (`GameplayStatics.GetPlayerCharacter` 0) :!pure true))
      (`/Game/ThirdPerson/Blueprints/Widgets/UI/W_InteractText.UpdateInteractText` _interacttextwidget "NewEnumerator3" (`self.HumanName`))
      (`UserWidget.AddToViewport` _interacttextwidget 0)
      (elif (== (`BlackboardComponent.GetValueAsInt` (`AIBlueprintHelperLibrary.GetBlackboard` null) "State") 0)
        (`/Game/ThirdPerson/Blueprints/Widgets/UI/W_InteractText.UpdateInteractText` _interacttextwidget_3 "NewEnumerator1" (`self.HumanName`))
        (`UserWidget.AddToViewport` _interacttextwidget_3 0)))))

(event `/Game/ThirdPerson/Blueprints/General/BPInterfaces/BPI_Interact.Fill`
  (if (`self.Dead?`)
    (`KismetArrayLibrary.Array_Clear` (`self.InventoryArray`))
    (for _array_element (`/Game/ThirdPerson/Blueprints/Widgets/Interfaces/W_BaseInterface.InterfaceSlotArray` (`/Game/ThirdPerson/Blueprints/BP_Character.ContainerWidget` (cast `/Game/ThirdPerson/Blueprints/BP_Character` (`GameplayStatics.GetPlayerCharacter` 0) :!pure true))) :!label _label
      (if (`/Game/ThirdPerson/Blueprints/Widgets/Slots/W_ContainerSlot.Filled?` _array_element)
        (`KismetArrayLibrary.Array_Add` (`self.InventoryArray`) (`/Game/ThirdPerson/Blueprints/Widgets/Slots/W_ContainerSlot.Item Info` _array_element))))
    (elif (`/Game/ThirdPerson/Blueprints/BP_Character.IsCrouching` (cast `/Game/ThirdPerson/Blueprints/BP_Character` (`GameplayStatics.GetPlayerCharacter` 0) :!pure true))
      (`KismetArrayLibrary.Array_Clear` (`self.InventoryArray`))
      (for _array_element_2 (`self.RemovedEquipmentArray`)
        (`KismetArrayLibrary.Array_Add` (`self.InventoryArray`) _array_element_2))
      (goto _label))))

(fn `GetFriendlyState`
  (params (InputTeamNumber :type Integer))
  (returns (FriendlyState :type Integer))
  (if (== InputTeamNumber (`self.TeamNumber`))
    (return 1)
    (elif (or (== InputTeamNumber 0) (== InputTeamNumber 1))
      (if (> (`/Game/ThirdPerson/Blueprints/BP_Character.Fine` (cast `/Game/ThirdPerson/Blueprints/BP_Character` (`GameplayStatics.GetPlayerCharacter` 0) :!pure true)) 0)
        (return -1)
        (else
          (return 0)))
      (elif (> InputTeamNumber 0)
        (return 0)
        (else
          (return -1))))))

(fn `GetTeam`
  (returns (OutputTeamNumber :type Integer))
  (return (`self.TeamNumber`)))

(fn `UserConstructionScript`
  (`parent.UserConstructionScript`))